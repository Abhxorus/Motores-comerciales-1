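; Traffic light actor that cycles its state through green, yellow and red.
; On BeginPlay, a looping timer fires AlternarLuz at a fixed interval, so every state lasts the same time.
; AlternarLuz switches on the EstadoActual enum, sets the next state and prints its name on screen.
; The graph only changes and prints the state, with no visual light update.
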(event Custom|AlternarLuz
  (switch Utilities|FlowControl|Switch|SwitchonE_EstadoSemaforo (Variables|Default|GetEstadoActual)
    (:NewEnumerator0
      (bind _output_get (Variables|Default|SetEstadoActual "NewEnumerator1"))
      (Development|PrintString (Utilities|String|EnumtoString _output_get)))
    (:NewEnumerator1
      (bind _output_get_2 (Variables|Default|SetEstadoActual "NewEnumerator2"))
      (Development|PrintString (Utilities|String|EnumtoString _output_get_2)))
    (:NewEnumerator2
      (bind _output_get_3 (Variables|Default|SetEstadoActual "NewEnumerator0"))
      (Development|PrintString (Utilities|String|EnumtoString _output_get_3)))))

(event EventBeginPlay
  (Utilities|Time|SetTimerbyEvent (delegate Custom|AlternarLuz) 5.0 true))

(event Collision|EventActorBeginOverlap
  (params (OtherActor :type Actor%20Object%20Reference)))

(event EventTick
  (params (DeltaSeconds :type Float%20%28single-precision%29)))

(fn ConstructionScript)