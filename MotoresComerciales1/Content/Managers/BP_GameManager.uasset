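; BP_GameManager periodically converts random pedestrian NPCs into chasers.
; After a startup delay, it starts a looping timer (RelojConversiones) that fires BuscarPeaton to gather every BP_SimpleNPC not flagged EsPerseguidor.
; It calls ActivarPerseguidor on a random candidate and clears the list, or stops the timer once no candidates remain.
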(event Custom|BuscarPeaton
  (bind _outactors (Actor|GetAllActorsOfClass "/Game/AI/BP_SimpleNPC.BP_SimpleNPC_C"))
  (for _array_element _outactors
    (if (not (Variables|/Game/AI/BP_SimpleNPC.BP_SimpleNPC_C|GetEsPerseguidor _array_element))
      (Utilities|Array|Add (Variables|Default|GetPeatonesDisponibles) _array_element)))
  (if (> (Utilities|Array|Length (Variables|Default|GetPeatonesDisponibles)) 0)
    (Default|ActivarPerseguidor (.OutItem (Utilities|Array|Random (Variables|Default|GetPeatonesDisponibles))))
    (Utilities|Array|Clear (Variables|Default|GetPeatonesDisponibles))
    (else
      (Utilities|Time|ClearandInvalidateTimerbyHandle (Variables|Default|GetRelojConversiones)))))

(event EventBeginPlay
  (Utilities|FlowControl|Delay 1e+01)
  (bind _returnvalue (Utilities|Time|SetTimerbyEvent (delegate Custom|BuscarPeaton) 5.0 true))
  (Variables|Default|SetRelojConversiones _returnvalue))

(event Collision|EventActorBeginOverlap
  (params (OtherActor :type Actor%20Object%20Reference)))

(event EventTick
  (params (DeltaSeconds :type Float%20%28single-precision%29)))

(fn ConstructionScript)